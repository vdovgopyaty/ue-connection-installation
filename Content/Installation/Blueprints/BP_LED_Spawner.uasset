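; BP_LED_Spawner builds a strip of BP_LED actors along a spline when play begins, as part of an installation.
; It spawns Quantity LEDs, evenly spaced over a hardcoded 1620-unit distance with integer step, aligned to the spline's world location and rotation.
; Each LED is stored by index in the LEDs array and starts at zero intensity.
; Once spawning finishes, it starts the OSC server on the level's BP_TD_OSC_In actor.
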(event EventBeginPlay
  (bind _spline (Variables|Default|GetSpline))
  (for _index (range 0 (- (Variables|Default|GetQuantity) 1))
    (bind _returnvalue (Game|SpawnActorfromClass "/Game/Installation/Blueprints/BP_LED.BP_LED_C" (Math|Transform|MakeTransform (Spline|GetLocationatDistanceAlongSpline _spline (Math|Conversions|ToFloat(Integer) (* _index (/ 1620 (Variables|Default|GetQuantity)))) "World") (Spline|GetRotationatDistanceAlongSpline _spline (Math|Conversions|ToFloat(Integer) (* _index (/ 1620 (Variables|Default|GetQuantity)))) "World") "1.000000,1.000000,1.000000") "Undefined" "MultiplyWithRoot" 0 0))
    (Utilities|Array|SetArrayElem (Variables|Default|GetLEDs) _index _returnvalue)
    (Default|SetIntensity _returnvalue 0.0))
  (bind _returnvalue_2 (Actor|GetActorOfClass "/Game/Installation/Blueprints/BP_TD_OSC_In.BP_TD_OSC_In_C"))
  (Default|OSCServerStart _returnvalue_2))

(fn ConstructionScript)