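; BP_TD_OSC_In is an OSC receiver that drives the intensity of BPLED actors in the level from incoming messages.
; OSCServerStart creates a listening OSC server, binds its message event and gathers all BPLED actors.
; Each /intensity message's floats set LED intensities by array index, relying on actor lookup order, and are printed for debugging.
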(event Custom|OnMsgReceived
  (params (Message :type OSC%20Message%20Structure%20%28by%20ref%29) (IPAddress :type String) (Port :type Integer))
  ;[1 1 1] Binding to Any Message
  (bind _returnvalue (Class|OSCManager|GetOSCMessageAddress Message))
  (bind _returnvalue_2 (Class|OSCManager|GetOSCAddressFullPath _returnvalue))
  (if (Class|KismetStringLibrary|MatchesWildcard _returnvalue_2 "/intensity" "IgnoreCase")
    (bind _values (Class|OSCManager|GetAllFloats Message))
    (for (_array_element _array_index) _values
      (Default|SetIntensity (Utilities|Array|Get(acopy) (stale Custom|OSCServerStart _outactors) _array_index) _array_element)
      (Development|PrintString (Utilities|String|Append "" _returnvalue_2 " " (Utilities|String|ToString(Float) _array_element))))))

(event Custom|OSCServerStart
  ;[1 1 1] Binding to Any Message
  (bind _returnvalue (Class|OSCManager|CreateOSCServer (Variables|Default|GetReceive%20IPAddress) (Variables|Default|GetPort) false true "UE_OSC" 0))
  (bind _output_get (Variables|Default|SetTD_OSC_Server _returnvalue))
  (EventDispatchers|AssignOnOscMessageReceived _output_get (delegate Custom|OnMsgReceived))
  (bind _outactors (Actor|GetAllActorsOfClass (Variables|Default|GetBP_LED))))

(fn ConstructionScript)